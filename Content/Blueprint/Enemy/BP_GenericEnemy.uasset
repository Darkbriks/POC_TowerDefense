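; BP_GenericEnemy is a generic enemy Blueprint that carries a LifeBar widget component.
; On BeginPlay it casts the component's widget to HUD_LifeBar and sets itself as that widget's Owner.
; Each Tick it rotates the bar in world space to face player 0's camera manager, and it destroys the component when the enemy is destroyed.
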(event EventBeginPlay
  (bind _ashud_life_bar (Utilities|Casting|CastToHUD_LifeBar (UserInterface|GetWidget (Variables|Default|GetLifeBar))))
  (Variables|/Game/Blueprint/Enemy/HUD_LifeBar.HUD_LifeBar_C|SetOwner _ashud_life_bar self))

(event EventTick
  (params (DeltaSeconds :type Float%20%28single-precision%29))
  (bind _lifebar (Variables|Default|GetLifeBar))
  (Transformation|SetWorldRotation _lifebar (Math|Rotator|FindLookatRotation (Transformation|GetWorldLocation _lifebar) (Transformation|GetWorldLocation (Variables|/Script/Engine.PlayerCameraManager|GetTransformComponent (Game|GetPlayerCameraManager 0)))) false false))

(event EventDestroyed
  (Components|DestroyComponent (Variables|Default|GetLifeBar)))

(fn ConstructionScript)